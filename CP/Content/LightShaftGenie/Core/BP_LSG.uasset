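; Configurable light shaft actor that renders a beam mesh with a dynamic material, built entirely in the construction script.
; It resets actor scale, picks a preset or custom mesh, then scales it by radius, axis offsets and length.
; It creates a single- or double-sided material instance, always double-sided for the Plane preset, and pushes grouped rays, opacity, color and noise settings into it.
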(event EventBeginPlay)

(event Collision|EventActorBeginOverlap
  (params (OtherActor :type Actor%20Object%20Reference)))

(event EventTick
  (params (DeltaSeconds :type Float%20%28single-precision%29)))

(fn ConstructionScript
  (Transformation|SetActorScale3D "1.000000,1.000000,1.000000")
  (CallFunction|UpdateShape)
  (|EditShape)
  (|BeamMaterialAssign))

(fn UpdateShape
  (bind _sm_beam (Variables|Default|GetSM_Beam))
  (Utilities|IsValid _sm_beam
    (:Is%20Valid
      (if (!= _sm_beam (.Mesh (Utilities|Struct|BreakFMeshCustom (Variables|LSG|Mesh|GetCustom%20Shape))))
        (if (.Enable (Utilities|Struct|BreakFMeshCustom (Variables|LSG|Mesh|GetCustom%20Shape))) :!label _label
          (Components|StaticMesh|SetStaticMesh (Variables|Default|GetSM_Beam) (.Mesh (Utilities|Struct|BreakFMeshCustom (Variables|LSG|Mesh|GetCustom%20Shape))))
          (else
            (switch Utilities|FlowControl|Switch|SwitchonEBeamMesh (.Presets (Utilities|Struct|BreakFMesh (Variables|LSG|Mesh|GetShape)))
              (:NewEnumerator0
                (Components|StaticMesh|SetStaticMesh (Variables|Default|GetSM_Beam) "/Game/LightShaftGenie/Meshes/SM_LightBeam_Cone.SM_LightBeam_Cone"))
              (:NewEnumerator1
                (Components|StaticMesh|SetStaticMesh (Variables|Default|GetSM_Beam) "/Game/LightShaftGenie/Meshes/SM_LightBeam_Cube_Tape.SM_LightBeam_Cube_Tape"))
              (:NewEnumerator2
                (Components|StaticMesh|SetStaticMesh (Variables|Default|GetSM_Beam) "/Game/LightShaftGenie/Meshes/SM_LightBeam_Cylinder.SM_LightBeam_Cylinder"))
              (:NewEnumerator3
                (Components|StaticMesh|SetStaticMesh (Variables|Default|GetSM_Beam) "/Game/LightShaftGenie/Meshes/SM_LightBeam_Cube.SM_LightBeam_Cube"))
              (:NewEnumerator4
                (Components|StaticMesh|SetStaticMesh (Variables|Default|GetSM_Beam) "/Game/LightShaftGenie/Meshes/SM_LightBeam_Plane.SM_LightBeam_Plane")))))))
    (:Is%20Not%20Valid
      (goto _label))))