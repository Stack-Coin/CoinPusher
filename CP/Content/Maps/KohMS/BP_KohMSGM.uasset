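; BP_KohMSGM, which by its name is the game mode for the KohMS map, sets up the player's UI at BeginPlay.
; It caches the player's BP_CPPlayerCharacter, then creates the stat, augment selection and item toast widgets and adds them to the viewport.
; HandleItemAcquired passes an acquired item to the toast widget, but its binding to the character's OnItemAcquired event is disconnected and never runs.
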(event Custom|HandleItemAcquired
  (params (AcquiredItem :type CP%20Item%20Data%20Structure))
  ;[0.15 0.15 0.15 0.5] 아이템 획득 이벤트 바인딩
  (Class|CPItemToastWidget|ShowToast (stale EventBeginPlay _returnvalue_3) AcquiredItem))

(event EventBeginPlay
  (bind _asbp_cpplayer_character (Utilities|Casting|CastToBP_CPPlayerCharacter (Game|GetPlayerCharacter 0)))
  (Variables|Default|SetCPPlayerCharacterRef _asbp_cpplayer_character)
  ;[0.15 0.15 0.15 0.5] 위젯 생성
  (bind _returnvalue (UserInterface|CreateWidget "/Game/Player/WBP_CPStatWidget.WBP_CPStatWidget_C"))
  (bind _returnvalue_2 (UserInterface|CreateWidget "/Game/Player/WBP_CPAugmentSelection.WBP_CPAugmentSelection_C"))
  (bind _returnvalue_3 (UserInterface|CreateWidget "/Game/Player/WBP_CPItemToast.WBP_CPItemToast_C"))
  (UserInterface|Viewport|AddtoViewport _returnvalue 0))

(fn ConstructionScript)